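; BP_Cannon is a cannon actor that repeatedly fires BP_Bullet projectiles on a timed cycle.
; Tick feeds an initial delay into a Duration delay, after which a bullet spawns at the Arrow component's location with configurable scale.
; Each shot plays CannonFireTimeline, which slides the barrel along its relative Y axis and loops back to the Duration delay when finished.
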(event `self.ReceiveTick`
  (params (DeltaSeconds :type "Float (single-precision)"))
  (`KismetSystemLibrary.Delay` 2.0)
  (`KismetSystemLibrary.Delay` (`self.Duration`) :!label _label)
  (`self.SpawnProjectile`)
  (bind (_direction _barrel_location) (`Timeline|Cannon Fire Timeline` :!via `PlayFromStart`)
    (:`Update`
      (`self.CannonBarrelMovement` _barrel_location))
    (:`Finished`
      (goto _label))))

(fn `CannonBarrelMovement`
  (params (CannonBarrelYLocation :type "Float (double-precision)"))
  (`SceneComponent.K2_SetRelativeLocation` (`self.Cannon_Barrel`) (`KismetMathLibrary.MakeVector` 0.0 CannonBarrelYLocation) false false))

(fn `SpawnProjectile`
  (`|SpawnActorFromClass` "/Game/Blueprints/Actors/Projectiles/BP_Bullet.BP_Bullet_C" (`KismetMathLibrary.MakeTransform` (`SceneComponent.K2_GetComponentLocation` (`self.Arrow`)) (struct) (`KismetMathLibrary.Conv_DoubleToVector` (`self.SpawnTransformScale`))) "Undefined" "OverrideRootScale" null null))

(fn `UserConstructionScript`)