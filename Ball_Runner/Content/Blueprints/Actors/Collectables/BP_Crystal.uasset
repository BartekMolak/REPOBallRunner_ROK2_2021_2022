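; BP_Crystal is a collectable crystal with a light that animates into the player on overlap, then destroys itself.
; When the player pawn overlaps it, the crystal caches its location, scale and light intensity.
; A timeline then drives separate curves that lerp it toward the pawn's live position while shrinking it to zero and fading the light out.
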(event `self.ReceiveActorBeginOverlap`
  (params (OtherActor :type "Actor Object Reference"))
  (if (== OtherActor (`GameplayStatics.GetPlayerPawn` 0))
    (`self.Start_Variables`)
    (bind (_direction _lerpmovement _lerpscale _lerplight) (`Timeline|TL_Blend_Alpha`)
      (:`Update`
        (`self.Location` _lerpmovement)
        (`self.Scale` _lerpscale)
        (`self.Light_Intensity` _lerplight))
      (:`Finished`
        (`self.K2_DestroyActor`)))))

(fn `Light_Intensity`
  (params (Alpha :type "Float (double-precision)"))
  (`LightComponent.SetIntensity` (`self.Crystal_Light`) (`KismetMathLibrary.Lerp` (`self.Crystal_Light_Intensity`) 0.0 Alpha)))

(fn `Location`
  (params (Alpha :type "Float (double-precision)"))
  (`self.K2_SetActorLocation` (`KismetMathLibrary.VLerp` (`self.Crystal_Location`) (`self.K2_GetActorLocation` (`GameplayStatics.GetPlayerPawn` 0)) Alpha)))

(fn `Scale`
  (params (Alpha :type "Float (double-precision)"))
  (`self.SetActorScale3D` (`KismetMathLibrary.VLerp` (`self.Crystal_Scale`) (0.0 0.0 0.0) Alpha)))

(fn `Start_Variables`
  (set `self.Crystal_Light_Intensity` (`LightComponentBase.Intensity` (`self.Crystal_Light`)))
  (set `self.Crystal_Scale` (`self.GetActorScale3D`))
  (set `self.Crystal_Location` (`self.K2_GetActorLocation`)))

(fn `UserConstructionScript`)